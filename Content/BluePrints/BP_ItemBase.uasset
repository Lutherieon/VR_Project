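; Base physics shop item that displays a dollar price and loses value when it takes hard impacts.
; Hits above an impulse threshold subtract random damage, play a sound and update the price, with a short random cooldown between hits.
; Surviving items in the cart report the loss to the BP_ShoppingCart found at BeginPlay.
; At zero value, the mesh swaps to a simulated Geometry Collection, which gets an impulse before the actor is destroyed.
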(event OnComponentHit(ItemMesh)
  (params (HitComponent :type Primitive%20Component%20Object%20Reference) (OtherActor :type Actor%20Object%20Reference) (OtherComp :type Primitive%20Component%20Object%20Reference) (NormalImpulse :type Vector :default "0, 0, 0") (Hit :type Hit%20Result%20Structure%20%28by%20ref%29))
  (if (>= (/ (Math|Vector|VectorLength NormalImpulse) 1e+02) 1e+01)
    (if (<= (Variables|Default|GetItemValue) 0)
      ;[1 1 1] BreakeItem
      (CallFunction|BreakeItem)
      (Utilities|FlowControl|DoOnce false
        (:Completed
          (Physics|AddImpulse (Variables|Default|GetGeometryCollection) "0.000000,0.000000,10.000000" "None" true)
          (Development|PrintString "Hello")
          (Utilities|FlowControl|Delay 2.0)
          (Actor|DestroyActor)))
      (elif (Variables|Default|GetHit?)
        (bind _output_get (Variables|Default|SetHitDamage (Math|Integer|Clamp(Integer) (Math|Random|RandomIntegerinRange (Variables|Default|GetMinHitDamage) (Variables|Default|GetMaxHitDamage)) 0 (Variables|Default|GetItemValue))))
        (bind _output_get_2 (Variables|Default|SetItemValue (Math|Integer|Clamp(Integer) (- (Variables|Default|GetItemValue) _output_get) 0 99999)))
        (Rendering|Components|TextRender|SetText (Variables|Default|GetPrice) (Utilities|Text|ToText(String) (Utilities|String|Append (Utilities|String|ToString(Integer) (Variables|Default|GetItemValue)) " $")))
        (Audio|PlaySound2D (Variables|Default|GetHitSound) 1.0 1.0 0.0 0 0)
        (if (<= (Variables|Default|GetItemValue) 0)
          ;[1 1 1] BreakeItem
          (CallFunction|BreakeItem)
          (Utilities|FlowControl|DoOnce false
            (:Completed
              (Physics|AddImpulse (Variables|Default|GetGeometryCollection) "0.000000,0.000000,10.000000" "None" true)
              (Development|PrintString "Hello")
              (Utilities|FlowControl|Delay 2.0)
              (Actor|DestroyActor)))
          (else
            (CallFunction|HitDelay)
            (if (Variables|Default|GetInCart?)
              (Class|BPIItemUpdate|ItemCostUpdate(Message) (Variables|Default|GetShoppingCartRef) _output_get _output_get_2))))))))

(event Custom|HitDelay
  (Variables|Default|SetHit? false)
  (Utilities|FlowControl|Delay (Math|Random|RandomFloatinRange 0.1 0.3))
  (Variables|Default|SetHit? true))

(event EventBeginPlay
  (Rendering|Components|TextRender|SetText (Variables|Default|GetPrice) (Utilities|Text|ToText(String) (Utilities|String|Append (Utilities|String|ToString(Integer) (Variables|Default|GetItemValue)) " $")))
  (bind _outactors (Actor|GetAllActorsOfClass "/Game/BluePrints/BP_ShoppingCart.BP_ShoppingCart_C"))
  (for _array_element _outactors
    (bind _asbp_shopping_cart (Utilities|Casting|CastToBP_ShoppingCart _array_element))
    (Variables|Default|SetShoppingCartRef _asbp_shopping_cart)))

(event Collision|EventActorBeginOverlap
  (params (OtherActor :type Actor%20Object%20Reference)))

(event EventReleaseItem
  (Physics|SetSimulatePhysics (Variables|Default|GetItemMesh) true))

(fn ConstructionScript)

(fn BreakeItem
  (bind _itemmesh (Variables|Default|GetItemMesh))
  (bind _geometrycollection (Variables|Default|GetGeometryCollection))
  (Rendering|SetVisibility _itemmesh false false)
  (Physics|SetSimulatePhysics _itemmesh false)
  (Physics|SetSimulatePhysics _geometrycollection true)
  (Rendering|SetVisibility _geometrycollection true false)
  (return))