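; Shopping cart actor that keeps a running dollar total and count of the items placed inside it, shown on a text render.
; Box overlaps with "Item"-tagged BP_ItemBase actors set their InCart flag and add or subtract their value, clamped.
; ItemCostUpdate subtracts damage from the total without clamping.
; HitDelay briefly blocks new additions for a random interval, while removals always register.
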(event OnComponentBeginOverlap(Box)
  (params (OverlappedComponent :type Primitive%20Component%20Object%20Reference) (OtherActor :type Actor%20Object%20Reference) (OtherComp :type Primitive%20Component%20Object%20Reference) (OtherBodyIndex :type Integer) (bFromSweep :type Boolean) (SweepResult :type Hit%20Result%20Structure%20%28by%20ref%29))
  ;[1 1 1] Item Overlap
  (if (Variables|Default|GetHit?)
    (if (Actor|ActorHasTag OtherActor "Item")
      (bind _asbp_item_base (Utilities|Casting|CastToBP_ItemBase OtherActor))
      (Variables|/Game/BluePrints/BP_ItemBase.BP_ItemBase_C|SetInCart? _asbp_item_base true)
      (bind _output_get (Variables|Default|SetTotalValue (Math|Integer|Clamp(Integer) (+ (Variables|Default|GetTotalValue) (Variables|/Game/BluePrints/BP_ItemBase.BP_ItemBase_C|GetItemValue _asbp_item_base)) 0 99999)))
      (Rendering|Components|TextRender|SetText (Variables|Default|GetTextRender) (Utilities|Text|ToText(String) (Utilities|String|Append (Utilities|String|ToString(Integer) _output_get) " $")))
      (Math|Integer|IncrementInt (Variables|Default|GetItemsInCart)))))

(event OnComponentEndOverlap(Box)
  (params (OverlappedComponent :type Primitive%20Component%20Object%20Reference) (OtherActor :type Actor%20Object%20Reference) (OtherComp :type Primitive%20Component%20Object%20Reference) (OtherBodyIndex :type Integer))
  ;[1 1 1] Item End Overlap
  (if (Actor|ActorHasTag OtherActor "Item")
    (bind _asbp_item_base (Utilities|Casting|CastToBP_ItemBase OtherActor))
    (Variables|/Game/BluePrints/BP_ItemBase.BP_ItemBase_C|SetInCart? _asbp_item_base false)
    (bind _output_get (Variables|Default|SetTotalValue (Math|Integer|Clamp(Integer) (- (Variables|Default|GetTotalValue) (Variables|/Game/BluePrints/BP_ItemBase.BP_ItemBase_C|GetItemValue _asbp_item_base)) 0 99999)))
    (Rendering|Components|TextRender|SetText (Variables|Default|GetTextRender) (Utilities|Text|ToText(String) (Utilities|String|Append (Utilities|String|ToString(Integer) _output_get) " $")))
    (Math|Integer|DecrementInt (Variables|Default|GetItemsInCart))))

(event Custom|HitDelay
  (Variables|Default|SetHit? false)
  (Utilities|FlowControl|Delay (Math|Random|RandomFloatinRange 0.1 0.3))
  (Variables|Default|SetHit? true))

(event EventBeginPlay
  (Rendering|Components|TextRender|SetText (Variables|Default|GetTextRender) (Utilities|Text|ToText(String) (Utilities|String|Append (Utilities|String|ToString(Integer) (Variables|Default|GetTotalValue)) " $"))))

(event Collision|EventActorBeginOverlap
  (params (OtherActor :type Actor%20Object%20Reference)))

(event EventItemCostUpdate
  (params (DamageValue :type Integer) (ItemValue :type Integer))
  (bind _output_get (Variables|Default|SetHitDamage DamageValue))
  (bind _output_get_2 (Variables|Default|SetTotalValue (- (Variables|Default|GetTotalValue) _output_get)))
  (Rendering|Components|TextRender|SetText (Variables|Default|GetTextRender) (Utilities|Text|ToText(String) (Utilities|String|Append (Utilities|String|ToString(Integer) _output_get_2) " $"))))

(fn ConstructionScript)