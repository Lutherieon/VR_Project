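; BP_Checkout is a checkout zone that counts item value against the quota held in VRGameMode and displays the remaining amount.
; After a short delay on BeginPlay, the TextRender shows the starting quota with a dollar sign.
; BP_ItemBase actors entering or leaving the Box adjust the local total and write directly to the game mode's quota.
; Each change updates the text, colors it success at zero or below and fail otherwise, and prints a debug message.
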(event OnComponentBeginOverlap(Box)
  (params (OverlappedComponent :type Primitive%20Component%20Object%20Reference) (OtherActor :type Actor%20Object%20Reference) (OtherComp :type Primitive%20Component%20Object%20Reference) (OtherBodyIndex :type Integer) (bFromSweep :type Boolean) (SweepResult :type Hit%20Result%20Structure%20%28by%20ref%29))
  (bind _asbp_item_base (Utilities|Casting|CastToBP_ItemBase OtherActor))
  (Variables|Default|SetValueInCheckOut (+ (Variables|/Game/BluePrints/BP_ItemBase.BP_ItemBase_C|GetItemValue _asbp_item_base) (Variables|Default|GetValueInCheckOut)))
  (bind _asvrgame_mode (Utilities|Casting|CastToVRGameMode (Game|GetGameMode)))
  (bind _output_get (Variables|/Game/VRTemplate/Blueprints/VRGameMode.VRGameMode_C|SetQuota _asvrgame_mode (- (Variables|/Game/VRTemplate/Blueprints/VRGameMode.VRGameMode_C|GetQuota _asvrgame_mode) (Variables|/Game/BluePrints/BP_ItemBase.BP_ItemBase_C|GetItemValue _asbp_item_base))))
  (Rendering|Components|TextRender|SetText (Variables|Default|GetTextRender) (Utilities|Text|ToText(Float) _output_get "HalfToEven"))
  (if (<= (Variables|/Game/VRTemplate/Blueprints/VRGameMode.VRGameMode_C|GetQuota _asvrgame_mode) 0.0)
    (Development|PrintString (Utilities|String|Append (Utilities|String|ToString(Float) (Variables|Default|GetValueInCheckOut)) " Succsess"))
    (Rendering|Components|TextRender|SetTextRenderColor (Variables|Default|GetTextRender) (Variables|Default|GetSuccses%20color))
    (else
      (Development|PrintString (Utilities|String|Append (Utilities|String|ToString(Float) (Variables|Default|GetValueInCheckOut)) " Fail"))
      (Rendering|Components|TextRender|SetTextRenderColor (Variables|Default|GetTextRender) (Variables|Default|GetFailedColor)))))

(event OnComponentEndOverlap(Box)
  (params (OverlappedComponent :type Primitive%20Component%20Object%20Reference) (OtherActor :type Actor%20Object%20Reference) (OtherComp :type Primitive%20Component%20Object%20Reference) (OtherBodyIndex :type Integer))
  (bind _asbp_item_base (Utilities|Casting|CastToBP_ItemBase OtherActor))
  (Variables|Default|SetValueInCheckOut (- (Variables|Default|GetValueInCheckOut) (Variables|/Game/BluePrints/BP_ItemBase.BP_ItemBase_C|GetItemValue _asbp_item_base)))
  (bind _asvrgame_mode (Utilities|Casting|CastToVRGameMode (Game|GetGameMode)))
  (bind _output_get (Variables|/Game/VRTemplate/Blueprints/VRGameMode.VRGameMode_C|SetQuota _asvrgame_mode (+ (Variables|/Game/VRTemplate/Blueprints/VRGameMode.VRGameMode_C|GetQuota _asvrgame_mode) (Variables|/Game/BluePrints/BP_ItemBase.BP_ItemBase_C|GetItemValue _asbp_item_base))))
  (Rendering|Components|TextRender|SetText (Variables|Default|GetTextRender) (Utilities|Text|ToText(Float) _output_get "HalfToEven"))
  (if (<= (Variables|/Game/VRTemplate/Blueprints/VRGameMode.VRGameMode_C|GetQuota _asvrgame_mode) 0.0)
    (Development|PrintString (Utilities|String|Append (Utilities|String|ToString(Float) (Variables|Default|GetValueInCheckOut)) " Succsess"))
    (Rendering|Components|TextRender|SetTextRenderColor (Variables|Default|GetTextRender) (Variables|Default|GetSuccses%20color))
    (else
      (Development|PrintString (Utilities|String|Append (Utilities|String|ToString(Float) (Variables|Default|GetValueInCheckOut)) " Fail"))
      (Rendering|Components|TextRender|SetTextRenderColor (Variables|Default|GetTextRender) (Variables|Default|GetFailedColor)))))

(event EventBeginPlay
  (Utilities|FlowControl|Delay 2.0)
  (bind _asvrgame_mode (Utilities|Casting|CastToVRGameMode (Game|GetGameMode)))
  (Rendering|Components|TextRender|SetText (Variables|Default|GetTextRender) (Utilities|Text|ToText(String) (Utilities|String|Append (Utilities|String|ToString(Text) (Utilities|Text|ToText(Float) (Variables|/Game/VRTemplate/Blueprints/VRGameMode.VRGameMode_C|GetQuota _asvrgame_mode) "HalfToEven")) "  $"))))

(event Collision|EventActorBeginOverlap
  (params (OtherActor :type Actor%20Object%20Reference)))

(event EventTick
  (params (DeltaSeconds :type Float%20%28single-precision%29)))

(fn ConstructionScript)