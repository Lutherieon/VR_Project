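; BP_GhostBase is a ghost enemy base that can attack, be grabbed and expose a patrol route through a getter.
; Attack plays a jump montage and fires OnAttackEnd on completion or interruption.
; GrabComponent events turn the mesh into a physics ragdoll while held, restoring collision and zeroing relative rotation on drop.
; Construction picks a random name, though the 0–4 range leaves the last four names unreachable.
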(event OnGrabbed(GrabComponent)
  (Physics|SetSimulatePhysics (Variables|Character|GetMesh) true)
  (Collision|SetCollisionProfileName (Variables|Character|GetMesh) "Ragdoll" true :!class /Script/Engine.PrimitiveComponent))

(event OnDropped(GrabComponent)
  (Physics|SetSimulatePhysics (Variables|Character|GetMesh) false)
  (Collision|SetCollisionProfileName (Variables|Character|GetMesh) "CharacterMesh" true :!class /Script/Engine.PrimitiveComponent)
  (Transformation|SetRelativeRotation (Variables|Character|GetMesh) "0, 0, 0" false false))

(event Custom|Attack
  (Animation|Montage|PlayMontage (Variables|Character|GetMesh) "/Game/Characters/Mannequins/Animations/Manny/MM_Jump_Montage.MM_Jump_Montage"
    (:OnCompleted
      _)
    (:OnInterrupted
      _))
  (Default|CallOnAttackEnd))

(event EventBeginPlay)

(event Collision|EventActorBeginOverlap
  (params (OtherActor :type Actor%20Object%20Reference)))

(fn ConstructionScript
  (switch int (Math|Random|RandomIntegerinRange 0 4)
    (:0
      (Variables|Default|SetGhostsName "John"))
    (:1
      (Variables|Default|SetGhostsName "Michael"))
    (:2
      (Variables|Default|SetGhostsName "Gabe"))
    (:3
      (Variables|Default|SetGhostsName "Rick"))
    (:4
      (Variables|Default|SetGhostsName "Jack"))
    (:5
      (Variables|Default|SetGhostsName "Jane"))
    (:6
      (Variables|Default|SetGhostsName "Kayle"))
    (:7
      (Variables|Default|SetGhostsName "Scarlett"))
    (:8
      (Variables|Default|SetGhostsName "Melissa"))))

(fn GetPatrolRoute
  (return (Variables|AI|References|GetPatrolRoute)))