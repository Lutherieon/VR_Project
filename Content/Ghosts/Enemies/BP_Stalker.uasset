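; BP_Stalker is a ghost enemy Blueprint that extends a parent class with a timed EMF signature.
; On BeginPlay it runs the parent logic, prints the ghost's name, then waits a random delay before spiking EMFLevel for a short window and resetting it to zero.
; The spike happens once, with no loop, and Tick and overlap events add no logic of their own.
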(event EventBeginPlay
  (|CallParentFunction)
  (Development|PrintString (Variables|Default|GetGhostsName))
  (Utilities|FlowControl|Sequence
    (:then_0
      (Utilities|FlowControl|Delay (Math|Random|RandomFloatinRange 5e+01 1.1e+02))
      (Variables|Default|SetEMFLevel 5.0)
      (Utilities|FlowControl|Delay 15.0)
      (Variables|Default|SetEMFLevel 0.0))))

(event Collision|EventActorBeginOverlap
  (params (OtherActor :type Actor%20Object%20Reference))
  (|CallParentFunction OtherActor) ; This node is disabled and will not be called.\nDrag off pins to build functionality.
)

(event EventTick
  (params (DeltaSeconds :type Float%20%28single-precision%29))
  (|CallParentFunction DeltaSeconds) ; This node is disabled and will not be called.\nDrag off pins to build functionality.
)

(fn ConstructionScript
  (|CallParentFunction))